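; Game manager that drives day progression and follower and reputation changes, storing the stats in GI_MaskGameInstance.
; Each action bumps a counter; passing the check advances the day and, after a delay, shows WBP_NewDay and refreshes computer-screen news unless it is the final day.
; Follower changes animate through a Timeline with color states, while reputation is clamped and re-banded.
; RevealFace uses another Timeline to swing the computer screen's camera yaw.
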(event `DelayIncreaseAndAcheck`
  (bind _gameinstance (`self.GameInstance`))
  (bind _gameinstance_2 (`self.GameInstance`))
  (`/Engine/EditorBlueprintResources/StandardMacros.IncrementInt` (`/Game/GI_MaskGameInstance.ActionCounter` _gameinstance)
    (:`  `
      (bind _isactionscomplete (`/Game/GI_MaskGameInstance.CheckActionCount` _gameinstance))
      (if _isactionscomplete
        (`/Game/GI_MaskGameInstance.IncrementDay ` _gameinstance_2)
        (set `self.GameState` "NewEnumerator1")
        (bind _isfinalday (`/Game/GI_MaskGameInstance.CheckForFinalDay ` _gameinstance_2))
        (`KismetSystemLibrary.Delay` 3.0)
        (`self.ShowDayWidget`)
        (if _isfinalday
          (`KismetSystemLibrary.PrintString` "EndOfDays")
          (else
            (`KismetSystemLibrary.PrintString` "Change to new day")
            (bind _outactors (`GameplayStatics.GetAllActorsOfClass` "/Game/Blueprints/BP_ComputerScreen.BP_ComputerScreen_C"))
            (for _array_element _outactors
              (`/Game/Blueprints/BP_ComputerScreen.DisplayNews` _array_element))))))))

(event `self.ReceiveBeginPlay`
  (bind _asgi_mask_game_instance (cast `/Game/GI_MaskGameInstance` (`GameplayStatics.GetGameInstance`)))
  (bind _output_get (set `self.GameInstance` _asgi_mask_game_instance))
  (`/Game/GI_MaskGameInstance.SetRepBand` _output_get)
  (bind _returnvalue (`GameplayStatics.GetActorOfClass` "/Game/Blueprints/BP_ComputerScreen.BP_ComputerScreen_C"))
  (set `self.ComputerScreenRef` _returnvalue))

(event `ShowDayWidget`
  (bind _returnvalue (`|CreateWidget` "/Game/Widgets/WBP_NewDay.WBP_NewDay_C" (`GameplayStatics.GetPlayerController` 0)))
  (bind _output_get (set `self.NewDayWidget` _returnvalue))
  (`UserWidget.AddToViewport` _output_get 0))

(event `LerpFollowerCount`
  (params (CurrentFollowerCount :type Integer) (NewFollowerCount :type Integer))
  (bind _gameinstance (`self.GameInstance`))
  (if (> NewFollowerCount CurrentFollowerCount)
    (set `/Game/GI_MaskGameInstance.FollowerCountColor` "NewEnumerator1" _gameinstance)
    (bind (_direction _alpha) (`Timeline|Timeline` :!via `PlayFromStart` :!label _label)
      (:`Update`
        (set `/Game/GI_MaskGameInstance.CurrentFollowerCount` (`KismetMathLibrary.FCeil` (`KismetMathLibrary.Lerp` (`KismetMathLibrary.Conv_IntToDouble` CurrentFollowerCount) (`KismetMathLibrary.Conv_IntToDouble` NewFollowerCount) _alpha)) (`self.GameInstance`)))
      (:`Finished`
        (set `/Game/GI_MaskGameInstance.FollowerCountColor` "NewEnumerator0" (`self.GameInstance`))))
    (else
      (set `/Game/GI_MaskGameInstance.FollowerCountColor` "NewEnumerator2" _gameinstance)
      (goto _label :!via `PlayFromStart`))))

(event `RevealFace`
  (bind (_direction _alpha) (`Timeline|Timeline_0` :!via `PlayFromStart`)
    (:`Update`
      (`SceneComponent.K2_SetRelativeRotation` (`/Game/Blueprints/BP_ComputerScreen.Camera` (`self.ComputerScreenRef`)) (`KismetMathLibrary.MakeRotator` 0.0 0.0 (`KismetMathLibrary.Lerp` -87.0 90.0 _alpha)) false false))))

(fn `ChangeFollowerCount`
  (params (FollowerChange :type Integer))
  (bind _currentfollowercount (`/Game/GI_MaskGameInstance.CurrentFollowerCount` (`self.GameInstance`)))
  (`self.LerpFollowerCount` _currentfollowercount (+ FollowerChange _currentfollowercount)))

(fn `ChangeRepCount`
  (params (RepChange :type Integer))
  (bind _gameinstance (`self.GameInstance`))
  (bind _maxrepscore (`/Game/GI_MaskGameInstance.MaxRepScore` _gameinstance))
  (bind _output_get (set `/Game/GI_MaskGameInstance.CurrentRepScore` (+ RepChange (`/Game/GI_MaskGameInstance.CurrentRepScore` _gameinstance)) _gameinstance))
  (if (> _output_get _maxrepscore)
    (set `/Game/GI_MaskGameInstance.CurrentRepScore` _maxrepscore _gameinstance)
    (elif (<= _output_get 0)
      (set `/Game/GI_MaskGameInstance.CurrentRepScore` 0 (`self.GameInstance`))))
  (`/Game/GI_MaskGameInstance.SetRepBand` _gameinstance))

(fn `Increase&CheckActionCount`
  (`self.DelayIncreaseAndAcheck`))

(fn `UserConstructionScript`)