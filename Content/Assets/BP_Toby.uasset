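; BP_Toby is an actor that animates an Img component and a Mask component with an idle bobbing motion.
; Each Tick drives both heights with sine waves over time since creation, each with its own speed and distance.
; When RemoveMask is true, the Mask instead slides down one unit per frame, independent of delta time.
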(event `self.ReceiveTick`
  (params (DeltaSeconds :type "Float (single-precision)"))
  (`|ExecutionSequence`
    (:`then_0`
      (`SceneComponent.K2_SetRelativeLocation` (`self.Img`) (`KismetMathLibrary.MakeVector` 0.0 0.0 (+ (`self.Return Value Location Z`) (* (`KismetMathLibrary.DegSin` (* (`self.GetGameTimeSinceCreation`) (`self.BobbingSpeed`))) (`self.BobbingDistance`)))) false false))
    (:`then_1`
      (if (`self.RemoveMask`)
        (`SceneComponent.K2_AddRelativeLocation` (`self.Mask`) (0.0 0.0 -1.0) false false)
        (else
          (`SceneComponent.K2_SetRelativeLocation` (`self.Mask`) (`KismetMathLibrary.MakeVector` 0.0 10.0 (+ (`self.Mask Return Value Location Z`) (* (`KismetMathLibrary.DegSin` (* (`self.GetGameTimeSinceCreation`) (`self.MaskBobbingSpeed`))) (`self.MaskBobbingDistance`)))) false false))))))

(event `CustomEvent`
  (params (DeltaSeconds :type "Float (single-precision)")))

(fn `UserConstructionScript`)