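; BP_TwitterScreen is an actor that hosts an in-game Twitter screen through a widget component showing WBP_TwitterWidget.
; On BeginPlay it binds to the widget's exit and option-chosen events.
; Exiting destroys the screen, while choosing an option first has the BP_ComputerScreen actor spawn a response window using BP_Outcome, then destroys it.
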(event `self.ReceiveBeginPlay`
  (bind _aswbp_twitter_widget (cast `/Game/Widgets/NewsWidgets/WBP_TwitterWidget` (`WidgetComponent.GetUserWidgetObject` (`self.Widget`))))
  (add `/Game/Widgets/NewsWidgets/WBP_TwitterWidget.OnExitTwitter` _aswbp_twitter_widget (delegate `Remove`))
  (add `/Game/Widgets/NewsWidgets/WBP_TwitterWidget.OnOptionChosen` _aswbp_twitter_widget (delegate `RemoveAndOption`)))

(event `RemoveAndOption`
  (bind _returnvalue (`GameplayStatics.GetActorOfClass` "/Game/Blueprints/BP_ComputerScreen.BP_ComputerScreen_C"))
  (`/Game/Blueprints/BP_ComputerScreen.SpawnResponseWindow` _returnvalue "/Game/BP_Outcome.BP_Outcome_C")
  (`self.K2_DestroyActor`))

(event `Remove`
  (`self.K2_DestroyActor`))

(fn `UserConstructionScript`)