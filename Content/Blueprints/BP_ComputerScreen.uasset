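; BP_ComputerScreen is an in-game computer screen actor that becomes the player's view target on BeginPlay and hosts windows as spawned actors.
; BeginPlay also calls DisplayNews, which triggers DelayedNews to spawn BP_NewsScreen above the screen after a short delay.
; Separate functions spawn Twittuh, Collab and response windows of a given class at fixed offsets from the screen.
; Twittuh and response windows share the CurrentTwittahScreen reference, while Collab uses CurrentCollabScreen.
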(event `DelayedNews`
  (bind _returnvalue (`self.GetTransform`))
  (`KismetSystemLibrary.Delay` 2.0)
  (`|SpawnActorFromClass` "/Game/Blueprints/BP_NewsScreen.BP_NewsScreen_C" (`KismetMathLibrary.MakeTransform` (`KismetMathLibrary.MakeVector` (- (.x (.location _returnvalue)) 0.0) (+ (.y (.location _returnvalue)) 0.0) (+ (.z (.location _returnvalue)) 155.0)) (.rotation _returnvalue) (.scale _returnvalue)) "Undefined" "MultiplyWithRoot" null null))

(event `self.ReceiveBeginPlay`
  (`PlayerController.SetViewTargetWithBlend` (`GameplayStatics.GetPlayerController` 0) self 0.0 "VTBlend_Linear" 0.0 false)
  (`self.DisplayNews`))

(fn `DisplayNews`
  (`self.DelayedNews`))

(fn `SpawnNewCollabWindow`
  (params (WidgetActorClass :type "Actor Class Reference"))
  (bind _returnvalue (`self.GetTransform`))
  (bind _returnvalue_2 (`|SpawnActorFromClass` WidgetActorClass (`KismetMathLibrary.MakeTransform` (`KismetMathLibrary.MakeVector` (+ (.x (.location _returnvalue)) 0.0) (+ (.y (.location _returnvalue)) -30.0) (+ (.z (.location _returnvalue)) 150.0)) (.rotation _returnvalue) (.scale _returnvalue)) "Undefined" "MultiplyWithRoot" null null))
  (set `self.CurrentCollabScreen` _returnvalue_2))

(fn `SpawnNewTwittuhWindow`
  (params (WidgetActorClass :type "Actor Class Reference"))
  (bind _returnvalue (`self.GetTransform`))
  (bind _returnvalue_2 (`|SpawnActorFromClass` WidgetActorClass (`KismetMathLibrary.MakeTransform` (`KismetMathLibrary.MakeVector` (- (.x (.location _returnvalue)) 0.0) (+ (.y (.location _returnvalue)) -30.0) (+ (.z (.location _returnvalue)) 150.0)) (.rotation _returnvalue) (.scale _returnvalue)) "Undefined" "MultiplyWithRoot" null null))
  (set `self.CurrentTwittahScreen` _returnvalue_2))

(fn `SpawnResponseWindow`
  (params (WidgetActorClass :type "Actor Class Reference"))
  (bind _returnvalue (`self.GetTransform`))
  (bind _returnvalue_2 (`|SpawnActorFromClass` WidgetActorClass (`KismetMathLibrary.MakeTransform` (`KismetMathLibrary.MakeVector` (+ (.x (.location _returnvalue)) 10.0) (+ (.y (.location _returnvalue)) -30.0) (+ (.z (.location _returnvalue)) 150.0)) (.rotation _returnvalue) (.scale _returnvalue)) "Undefined" "MultiplyWithRoot" null null))
  (set `self.CurrentTwittahScreen` _returnvalue_2))

(fn `UserConstructionScript`)